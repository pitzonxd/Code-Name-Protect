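; Tower defense grid actor that sizes its plane from Cols and Rows and serves as the spawner and registry for enemies.
; Pressing Z spawns a batch of StandardEnemy_BP AI running Enemy_BT, re-rolling random HitBox points until each lands outside the plane.
; Spawned enemies go into AllEnemies, which backs a nearest-enemy-within-radius query for towers and is pruned when enemies die.
; CalculateOrigin, called at BeginPlay, derives an inset corner origin from the plane bounds.
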(event Custom|RemoveDeadEnemy
  (params (NewParam :type Standard%20Enemy%20BP%20Object%20Reference))
  ;[1 1 1] Remove dead enemy (Called from StandartEemyBP)
  (Actor|DestroyActor NewParam)
  (Utilities|Array|RemoveItem (Variables|Default|GetAllEnemies) NewParam))

(event EventBeginPlay
  (|CalculateOrigin))

(event Input|KeyboardEvents|Z
  (params (Key :type Key%20Structure))
  (bind _hitbox (Variables|Default|GetHitBox))
  (bind _plane (Variables|Default|GetPlane))
  (bind (_origin _boxextent) (Collision|GetComponentBounds _plane))
  (bind (_origin_2 _boxextent_2) (Collision|GetComponentBounds _hitbox))
  (:Pressed
    (while (< (Variables|Default|GetspawnedEnemies) (Variables|Default|GetEnemiesToSpawn))
      (Variables|Default|SetTargetSpawnLocation (Math|Vector|MakeVector (+ (.x _origin_2) (* (.x _boxextent_2) (Math|Random|RandomFloatinRange -0.95 0.95))) (+ (.y _origin_2) (* (.y _boxextent_2) (Math|Random|RandomFloatinRange -0.95 0.95))) (.z (.Origin (Collision|GetComponentBounds (Variables|Default|GetPlane))))))
      (if (not (and (and (< (.x (Variables|Default|GetTargetSpawnLocation)) (+ (.x _origin) (.x _boxextent))) (> (.x (Variables|Default|GetTargetSpawnLocation)) (- (.x _origin) (.x _boxextent)))) (and (< (.y (Variables|Default|GetTargetSpawnLocation)) (+ (.y _origin) (.y _boxextent))) (> (.y (Variables|Default|GetTargetSpawnLocation)) (- (.y _origin) (.y _boxextent))))))
        (bind _returnvalue (AI|SpawnAIFromClass "/Game/TowerDefense/Enemies/StandardEnemy_BP.StandardEnemy_BP_C" "/Game/TowerDefense/Enemies/Enemy_BT.Enemy_BT" (Variables|Default|GetTargetSpawnLocation) "0, 0, 0" false 0))
        (bind _asstandard_enemy_bp (Utilities|Casting|CastToStandardEnemy_BP _returnvalue))
        (Utilities|Array|Add (Variables|Default|GetAllEnemies) _asstandard_enemy_bp)
        (Math|Integer|IncrementInt (Variables|Default|GetspawnedEnemies))))
    (Variables|Default|SetspawnedEnemies 0)))

(fn ConstructionScript
  (bind _rows (Variables|Default|Getrows))
  (bind _plane (Variables|Default|GetPlane))
  (bind _returnvalue (* _rows 2))
  (bind _returnvalue_2 (Math|Conversions|ToFloat(Integer) _returnvalue))
  (Transformation|SetWorldTransform _plane (Math|Transform|MakeTransform (.location (Transformation|GetWorldTransform _plane)) "0, 0, 0" (Math|Vector|MakeVector (Math|Conversions|ToFloat(Integer) (* (Variables|Default|Getcols) 2)) _returnvalue_2 _returnvalue_2)) false false))

(fn GetClosestEnemytoTower
  (params (Tower :type Target%20BP%20Object%20Reference) (damageradius :type Float%20%28single-precision%29))
  (bind _allenemies (Variables|Default|GetAllEnemies))
  (LocalVariables|SettmpTower Tower)
  (LocalVariables|SetdamageRadiusTmp damageradius)
  (if (== (Utilities|Array|Length (Variables|Default|GetAllEnemies)) 0)
    (return 0)
    (else
      (LocalVariables|SetClosestEnemy (Utilities|Array|Get(acopy) _allenemies))
      (for _index (range 1 (- (Utilities|Array|Length _allenemies) 1))
        (if (< (Transformation|GetDistanceTo (LocalVariables|GettmpTower) (Utilities|Array|Get(acopy) (Variables|Default|GetAllEnemies) _index)) (Transformation|GetDistanceTo (LocalVariables|GettmpTower) (LocalVariables|GetClosestEnemy)))
          (LocalVariables|SetClosestEnemy (Utilities|Array|Get(acopy) (Variables|Default|GetAllEnemies) _index))))
      (if (<= (Transformation|GetDistanceTo (LocalVariables|GetClosestEnemy) (LocalVariables|GettmpTower)) (LocalVariables|GetdamageRadiusTmp))
        (return (LocalVariables|GetClosestEnemy))
        (else
          (return 0))))))