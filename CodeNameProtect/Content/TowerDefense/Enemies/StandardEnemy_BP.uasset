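; StandardEnemy_BP is a tower defense enemy with health that dies when damage depletes it.
; The construction script sets CurrentHealth to MaxHealth, and AnyDamage subtracts incoming damage from it.
; At zero or below, it casts the player character to Char_Christophe, tells that character's GridReference to remove the dead enemy, then destroys itself.
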(event Game|Damage|EventAnyDamage
  (params (Damage :type Float%20%28single-precision%29) (DamageType :type Damage%20Type%20Object%20Reference) (InstigatedBy :type Controller%20Object%20Reference) (DamageCauser :type Actor%20Object%20Reference))
  (Variables|Default|SetcurrentHealth (- (Variables|Default|GetcurrentHealth) Damage))
  (if (<= (Variables|Default|GetcurrentHealth) 0.0)
    (bind _aschar_emma_copy (Utilities|Casting|CastToChar_Christophe (Game|GetPlayerCharacter 0)))
    (Default|RemoveDeadEnemy (Variables|/Game/ThirdPersonBP/Blueprints/Char_Christophe.Char_Christophe_C|GetGridReference _aschar_emma_copy) self)
    (Actor|DestroyActor)))

(fn ConstructionScript
  (Variables|Default|SetcurrentHealth (Variables|Default|GetmaxHealth)))