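; Placeable tower-defense wall trap that damages a StandardEnemy_BP entering its hitbox and fires spikes.
; A timeline extends the spikes, holds them for the activation time, then reverses and waits out a cooldown before re-arming.
; While unplaced, Tick allows placement only when unblocked, touching a Wall_BP and free of mesh overlaps, tinting the base mesh blueprint or red.
; It extends parent placement logic, restoring normal materials once placed.
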(event OnComponentBeginOverlap(Hitbox)
  (params (OverlappedComponent :type Primitive%20Component%20Object%20Reference) (OtherActor :type Actor%20Object%20Reference) (OtherComp :type Primitive%20Component%20Object%20Reference) (OtherBodyIndex :type Integer) (bFromSweep :type Boolean) (SweepResult :type Hit%20Result%20Structure%20%28by%20ref%29))
  ;[1 1 1] Apply damage to overlaping enemy
  (if (Variables|Default|GetcanBeTriggered)
    (bind _asstandard_enemy_bp (Utilities|Casting|CastToStandardEnemy_BP OtherActor))
    (Game|Damage|ApplyDamage _asstandard_enemy_bp (Variables|Default|Getdamage) 0 0)
    (CallFunction|EnableTrap)))

(event Custom|EnableTrap
  ;[1 1 1] Enable Disable trap
  (Variables|Default|SetcanBeTriggered false)
  (Variables|Default|Setenabled true)
  (bind _newtrack_0 (Timeline|EnableDisableSpikes PlayFromStart)
    (:Update
      (Transformation|SetRelativeLocation (Variables|Default|GetSpikes) (Math|Vector|MakeVector 0.0 0.0 (+ (* _newtrack_0 5e+01) 3e+01)) false false))
    (:Finished
      (if (Variables|Default|Getenabled)
        (Utilities|FlowControl|Delay (Variables|Default|GetactivationTime))
        (CallFunction|DisableTrap)
        (else
          (Utilities|FlowControl|Delay (Variables|Default|Getcooldown))
          (Variables|Default|SetcanBeTriggered true))))))

(event Custom|DisableTrap
  ;[1 1 1] Enable Disable trap
  (Variables|Default|Setenabled false)
  (bind _newtrack_0 (Timeline|EnableDisableSpikes ReverseFromEnd)
    (:Update
      (Transformation|SetRelativeLocation (Variables|Default|GetSpikes) (Math|Vector|MakeVector 0.0 0.0 (+ (* _newtrack_0 5e+01) 3e+01)) false false))
    (:Finished
      (if (Variables|Default|Getenabled)
        (Utilities|FlowControl|Delay (Variables|Default|GetactivationTime))
        (CallFunction|DisableTrap)
        (else
          (Utilities|FlowControl|Delay (Variables|Default|Getcooldown))
          (Variables|Default|SetcanBeTriggered true))))))

(event EventTick
  (params (DeltaSeconds :type Float%20%28single-precision%29))
  (bind _staticmesh (Variables|Default|GetStaticMesh))
  ;[1 1 1] Set material when in building mode
  (|CallParentFunction DeltaSeconds)
  (if (not (Variables|Default|Getplaced))
    (bind _aschar_christophe (Utilities|Casting|CastToChar_Christophe (Game|GetPlayerCharacter 0)))
    (if (Variables|/Game/ThirdPersonBP/Blueprints/Char_Christophe.Char_Christophe_C|GetplacementBlocked _aschar_christophe)
      (Rendering|Material|SetMaterial _staticmesh 0 "/Game/TowerDefense/Materials/RedMaterial.RedMaterial" :!label _label)
      (Variables|Default|SetcanBePlaced false)
      (elif (== (Utilities|Array|Length (Collision|GetOverlappingActors (Variables|Default|GetWallChecker) "/Game/TowerDefense/Assets/Wall_BP.Wall_BP_C" :!class /Script/Engine.PrimitiveComponent)) 0)
        (goto _label)
        (elif (== (Utilities|Array|Length (Collision|GetOverlappingActors (Variables|Default|GetStaticMesh) 0 :!class /Script/Engine.PrimitiveComponent)) 0)
          (Rendering|Material|SetMaterial _staticmesh 0 "/Game/TowerDefense/Materials/BlueprintMaterial.BlueprintMaterial")
          (Variables|Default|SetcanBePlaced true)
          (else
            (goto _label)))))))

(event EventPlaceTarget
  (params (Target :type Target%20BP%20Class%20Reference))
  (bind _material (Variables|Default|GetMaterial))
  ;[1 1 1] Set material when placed
  (|CallParentFunction Target)
  (Rendering|Material|SetMaterial (Variables|Default|GetStaticMesh) 0 _material)
  (Rendering|Material|SetMaterial (Variables|Default|GetSpikes) 0 _material))

(event EventBeginPlay
  ;[1 1 1] Set rotation, so that the player sees the front of the trap when spawned
  (|CallParentFunction)
  (Variables|/Game/ThirdPersonBP/Blueprints/Char_Christophe.Char_Christophe_C|Setrotation (Variables|Default|GetCharacterReference) 2.7e+02))

(fn ConstructionScript
  (Variables|Default|SetTrapLocation (Transformation|GetWorldLocation (Variables|Default|GetSpikes))))