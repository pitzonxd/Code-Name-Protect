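; Placeable spike trap for a tower defense game that damages a StandardEnemy_BP overlapping its hitbox while armed.
; Triggering damages only that enemy, disarms the trap and raises the spikes via a timeline.
; The timeline's Finished branches on Enabled: hold for ActivationTime then reverse, or wait Cooldown then re-arm.
; Placement applies the material to base and spikes; spike relative Z is offset from a construction-time world Z.
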(event OnComponentBeginOverlap(Hitbox)
  (params (OverlappedComponent :type Primitive%20Component%20Object%20Reference) (OtherActor :type Actor%20Object%20Reference) (OtherComp :type Primitive%20Component%20Object%20Reference) (OtherBodyIndex :type Integer) (bFromSweep :type Boolean) (SweepResult :type Hit%20Result%20Structure%20%28by%20ref%29))
  (if (Variables|Default|GetcanBeTriggered)
    (bind _asstandard_enemy_bp (Utilities|Casting|CastToStandardEnemy_BP OtherActor))
    (Game|Damage|ApplyDamage _asstandard_enemy_bp (Variables|Default|Getdamage) 0 0)
    (CallFunction|EnableTrap)))

(event Custom|EnableTrap
  (Variables|Default|SetcanBeTriggered false)
  (Variables|Default|Setenabled true)
  (bind _newtrack_0 (Timeline|EnableDisableSpikes PlayFromStart)
    (:Update
      (Transformation|SetRelativeLocation (Variables|Default|GetSpikes) (Math|Vector|MakeVector 0.0 0.0 (+ (* _newtrack_0 5e+01) (.z (Variables|Default|GetTrapLocation)))) false false))
    (:Finished
      (if (Variables|Default|Getenabled)
        (Utilities|FlowControl|Delay (Variables|Default|GetactivationTime))
        (CallFunction|DisableTrap)
        (else
          (Utilities|FlowControl|Delay (Variables|Default|Getcooldown))
          (Variables|Default|SetcanBeTriggered true))))))

(event Custom|DisableTrap
  (Variables|Default|Setenabled false)
  (bind _newtrack_0 (Timeline|EnableDisableSpikes ReverseFromEnd)
    (:Update
      (Transformation|SetRelativeLocation (Variables|Default|GetSpikes) (Math|Vector|MakeVector 0.0 0.0 (+ (* _newtrack_0 5e+01) (.z (Variables|Default|GetTrapLocation)))) false false))
    (:Finished
      (if (Variables|Default|Getenabled)
        (Utilities|FlowControl|Delay (Variables|Default|GetactivationTime))
        (CallFunction|DisableTrap)
        (else
          (Utilities|FlowControl|Delay (Variables|Default|Getcooldown))
          (Variables|Default|SetcanBeTriggered true))))))

(event EventPlaceTarget
  (params (Target :type Target%20BP%20Class%20Reference))
  (bind _material (Variables|Default|GetMaterial))
  ;[1 1 1] Set material
  (|CallParentFunction Target)
  (Rendering|Material|SetMaterial (Variables|Default|GetStaticMesh) 0 _material)
  (Rendering|Material|SetMaterial (Variables|Default|GetSpikes) 0 _material))

(fn ConstructionScript
  (Variables|Default|SetTrapLocation (Transformation|GetWorldLocation (Variables|Default|GetSpikes))))