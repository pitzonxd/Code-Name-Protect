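; Tower defense tower that, once placed, continuously damages the enemy its grid picks as closest.
; Placement runs the parent logic, then sets the mesh material.
; Each Tick it queries the player character's grid reference for that enemy and applies damage scaled by frame time and a multiplier.
; A line trace to the enemy draws a one-frame debug line as the shot; its hit result is unused, so obstacles don't block damage.
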(event EventTick
  (params (DeltaSeconds :type Float%20%28single-precision%29))
  (bind _self self)
  (bind _returnvalue (Transformation|GetActorLocation _self))
  (bind _aschar_emma_copy (Utilities|Casting|CastToChar_Emma_Copy (Game|GetPlayerCharacter 0)))
  (bind _enemy (Default|GetClosestEnemytoTarget (Variables|/Game/ThirdPersonBP/Blueprints/Char_Emma_Copy.Char_Emma_Copy_C|GetGridReference _aschar_emma_copy) self))
  (if (!= _enemy 0)
    (Collision|LineTraceByChannel (Math|Vector|MakeVector (.x _returnvalue) (.y _returnvalue) 3e+02) (Math|Vector|MakeVector (.x (Transformation|GetActorLocation _enemy)) (.y (Transformation|GetActorLocation _enemy)) 1.5e+02) "TraceTypeQuery1" false 0 "ForOneFrame")
    (Game|Damage|ApplyDamage _enemy (* DeltaSeconds (Variables|Default|GetdamageMultiplier)) 0 0)))

(event EventPlaceTarget
  (params (Target :type Target%20BP%20Class%20Reference))
  (|CallParentFunction Target)
  (Rendering|Material|SetMaterial (Variables|Default|GetStaticMesh) 0 (Variables|Default|GetMaterial)))

(fn ConstructionScript)