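; Placeable tower-defense actor that acts as a build preview following the player's aim and spawns the placed structure.
; Each tick, towers snap to their referenced wall, while other unplaced types snap the character's hit point to a 200-unit grid.
; Except for wall traps, overlaps or blocked placement turn the preview red and unplaceable.
; PlaceTarget spawns the given class with blocking collision, marks it placed and registers towers with their wall.
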(event Custom|SetGrid
  (params (GridReference :type Grid%20BP%20Object%20Reference))
  (Variables|Default|SetGridReference GridReference))

(event Custom|PlaceTarget
  (params (Target :type Target%20BP%20Class%20Reference))
  (bind _wallreference (Variables|Default|GetWallReference))
  (if (Utilities|Enum|Equal(Enum) (Variables|Default|Gettype) "tower")
    (bind _returnvalue (Game|SpawnActorfromClass Target (Math|Transform|MakeTransform (Transformation|GetActorLocation _wallreference) (Math|Rotator|MakeRotator 0.0 0.0 (Variables|/Game/ThirdPersonBP/Blueprints/Char_Christophe.Char_Christophe_C|Getrotation (Variables|Default|GetCharacterReference))) "1,1,1") "Undefined" 0 0))
    (CallFunction|SetTower _wallreference _returnvalue)
    (Collision|SetCollisionResponsetoAllChannels (Variables|Target_BP_C|GetStaticMesh _returnvalue) "ECR_Block")
    (Variables|Target_BP_C|Setplaced _returnvalue true)
    (else
      (bind _returnvalue_2 (Game|SpawnActorfromClass Target (Math|Transform|MakeTransform (Variables|Default|GetLocation) (Math|Rotator|MakeRotator 0.0 0.0 (Variables|/Game/ThirdPersonBP/Blueprints/Char_Christophe.Char_Christophe_C|Getrotation (Variables|Default|GetCharacterReference))) "1.000000,1,1") "Undefined" 0 0))
      (Collision|SetCollisionResponsetoAllChannels (Variables|Target_BP_C|GetStaticMesh _returnvalue_2) "ECR_Block")
      (Variables|Target_BP_C|Setplaced _returnvalue_2 true))))

(event Custom|SetTower
  (params (TowerReference :type Target%20BP%20Object%20Reference))
  (Variables|Default|SetTowerReference TowerReference))

(event Custom|SetWall
  (params (WallReference :type Wall%20BP%20Object%20Reference))
  (Variables|Default|SetWallReference WallReference))

(event EventTick
  (params (DeltaSeconds :type Float%20%28single-precision%29))
  (bind _characterreference (Variables|Default|GetCharacterReference))
  (bind _gridreference (Variables|Default|GetGridReference))
  (bind _staticmesh (Variables|Default|GetStaticMesh))
  (bind _hitlocation (Variables|/Game/ThirdPersonBP/Blueprints/Char_Christophe.Char_Christophe_C|GetHitLocation _characterreference))
  (bind _realorigin (Variables|/Game/TowerDefense/Grid_BP.Grid_BP_C|GetRealOrigin _gridreference))
  (bind _returnvalue (- _hitlocation _realorigin))
  (if (Utilities|Enum|Equal(Enum) (Variables|Default|Gettype) "tower")
    (bind _wallreference (Variables|Default|GetWallReference)
      (:then
        (Transformation|SetActorLocation (Transformation|GetActorLocation _wallreference) false false)
        (if (not (Utilities|Enum|Equal(Enum) (Variables|Default|Gettype self) "walltrap")) :!label _label
          (if (== (Utilities|Array|Length (Collision|GetOverlappingActors self 0 :!class /Script/Engine.Actor)) 0)
            (if (Variables|/Game/ThirdPersonBP/Blueprints/Char_Christophe.Char_Christophe_C|GetplacementBlocked (Variables|Default|GetCharacterReference))
              (Rendering|Material|SetMaterial _staticmesh 0 "/Game/TowerDefense/Materials/RedMaterial.RedMaterial" :!label _label_2)
              (Variables|Default|SetcanBePlaced false)
              (else
                (Rendering|Material|SetMaterial _staticmesh 0 "/Game/TowerDefense/Materials/BlueprintMaterial.BlueprintMaterial")
                (Variables|Default|SetcanBePlaced true)))
            (else
              (goto _label_2)))))
      (:else))
    (else
      (Variables|Default|GetGridReference
        (:then
          (if (not (Variables|Default|Getplaced))
            (bind _output_get (Variables|Default|SetLocation (+ (Math|Vector|MakeVector (* (Math|Conversions|ToFloat(Integer) (Math|Float|Round (/ (.x _returnvalue) 2e+02))) 2e+02) (* (Math|Conversions|ToFloat(Integer) (Math|Float|Round (/ (.y _returnvalue) 2e+02))) 2e+02) (.z _returnvalue)) _realorigin)))
            (Transformation|SetActorLocation _output_get false false)
            (goto _label)))
        (:else)))))

(event EventBeginPlay
  (bind _aschar_christophe (Utilities|Casting|CastToChar_Christophe (Game|GetPlayerCharacter 0)))
  (Variables|Default|SetCharacterReference _aschar_christophe))

(fn ConstructionScript)