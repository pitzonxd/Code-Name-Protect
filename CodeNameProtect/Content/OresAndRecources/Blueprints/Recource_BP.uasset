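; Recource_BP is a resource Blueprint, likely an ore or similar harvestable, that yields random drops from four breakable parts.
; The construction script fills the Drops array with a random count per part, bounded by MinDropsPerPart and MaxDropsPerPart.
; Four GetDropsPart functions each flag their part in PartsDestroyed and return that part's pre-rolled count, leaving spawning and visuals outside these graphs.
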(fn ConstructionScript
  (for _index (range 0 3)
    (Utilities|Array|SetArrayElem (Variables|Default|GetDrops) _index (Math|Random|RandomIntegerinRange (Variables|Default|GetminDropsPerPart) (Variables|Default|GetmaxDropsPerPart)))))

(fn GetDropsPart1
  (Utilities|Array|SetArrayElem (Variables|Default|GetpartsDestroyed) 0 true)
  (return (Utilities|Array|Get(acopy) (Variables|Default|GetDrops))))

(fn GetDropsPart2
  (Utilities|Array|SetArrayElem (Variables|Default|GetpartsDestroyed) 1 true)
  (return (Utilities|Array|Get(acopy) (Variables|Default|GetDrops) 1)))

(fn GetDropsPart3
  (Utilities|Array|SetArrayElem (Variables|Default|GetpartsDestroyed) 2 true)
  (return (Utilities|Array|Get(acopy) (Variables|Default|GetDrops) 2)))

(fn GetDropsPart4
  (Utilities|Array|SetArrayElem (Variables|Default|GetpartsDestroyed) 3 true)
  (return (Utilities|Array|Get(acopy) (Variables|Default|GetDrops) 3)))