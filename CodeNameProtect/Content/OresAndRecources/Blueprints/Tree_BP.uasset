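; Tree actor that falls over when triggered and turns into a Wood pickup.
; StartFalling derives a 2D direction from the hit location relative to the trunk and uses it to drive a RotatingMovement component.
; A per-frame Delay loop accelerates the rotation until HitCollider overlaps more than one actor.
; The tree then destroys itself and spawns Wood at its BeginPlay location with a random quantity within its drop range.
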(event Custom|StartFalling
  (params (HitLocation :type Vector))
  (bind _returnvalue (Utilities|Time|GetWorldDeltaSeconds))
  (bind _tree (Variables|Default|GetTree))
  (bind _returnvalue_2 (Transformation|GetWorldLocation _tree))
  (bind _returnvalue_3 (- HitLocation _returnvalue_2))
  (bind _returnvalue_4 (Class|KismetMathLibrary|VectorNormal2D _returnvalue_3 0.0001))
  (Variables|Default|Setfalling true)
  (Variables|Default|SetFallDirection (Math|Vector2D|MakeVector2D (.x _returnvalue_4) (.y _returnvalue_4)))
  (if (> (Utilities|Array|Length (Collision|GetOverlappingActors (Variables|Default|GetHitCollider) 0 :!class /Script/Engine.PrimitiveComponent)) 1) :!label _label
    (Variables|/Script/Engine.RotatingMovementComponent|SetRotationRate (Variables|Default|GetRotatingMovement) (Math|Rotator|MakeRotator 0.0 0.0 0.0))
    (Actor|DestroyActor)
    (bind _returnvalue_5 (Game|SpawnActorfromClass "/Game/ThirdPersonBP/Blueprints/Potions/Potions/BP/Wood.Wood_C" (Math|Transform|MakeTransform (Variables|Default|GetActorLocation) "0, 0, 0" "1,1,1") "Undefined" 0 0))
    (Variables|/Game/ThirdPersonBP/Blueprints/Potions/Potions/BP/Healtpotion.Healtpotion_C|SetQuantity _returnvalue_5 (Math|Random|RandomIntegerinRange (Variables|Default|GetminDropPieces) (Variables|Default|GetmaxDropPieces)))
    (else
      (Utilities|FlowControl|Delay _returnvalue)
      (bind _output_get (Variables|Default|Setspeed (+ (Variables|Default|Getspeed) (* _returnvalue (Variables|Default|Getspeed)))))
      (Variables|/Script/Engine.RotatingMovementComponent|SetRotationRate (Variables|Default|GetRotatingMovement) (Math|Rotator|MakeRotator (.x (* (Variables|Default|GetFallDirection) _output_get)) (.y (* (Variables|Default|GetFallDirection) _output_get)) 0.0))
      (goto _label))))

(event EventBeginPlay
  (Variables|/Script/Engine.RotatingMovementComponent|SetRotationRate (Variables|Default|GetRotatingMovement) (Math|Rotator|MakeRotator 0.0 0.0 0.0))
  (Variables|Default|SetActorLocation (Transformation|GetActorLocation)))

(fn ConstructionScript)