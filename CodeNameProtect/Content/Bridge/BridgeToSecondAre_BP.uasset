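; Buildable bridge Blueprint that tracks donated items against a required list, seeded into CurrentCompletion at BeginPlay.
; Interact passes each inventory slot to ConstructOnServer, which only prints the player's name, then prints "Bridge built" if CheckIfCompleted passes.
; AddItemsToConstructions matches DataTable row names, caps deposits at the remainder and deducts player slots, but is never called here.
; CheckIfCompleted returns after testing only the first requirement.
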(event Custom|Server
  (Development|PrintString (Utilities|String|ToString(Integer) (.Amount (Utilities|Struct|BreakS_Slots (Utilities|Array|Get(acopy) (Variables|Default|GetCurrentCompletion)))))))

(event Custom|ConstructOnServer
  (params (AddedItem :type S%20Slots%20Structure) (PlayerReference :type Char%20Emma%20Object%20Reference))
  (Development|PrintString (Utilities|GetDisplayName PlayerReference)))

(event EventBeginPlay
  (for _array_element (Variables|Default|GetRequiredItemsForCompletion)
    (Utilities|Array|Add (Variables|Default|GetCurrentCompletion) (Utilities|Struct|MakeS_Slots (.Item (Utilities|Struct|BreakS_Slots _array_element))))))

(event EventTick
  (params (DeltaSeconds :type Float%20%28single-precision%29)))

(event EventInteract
  (params (PCRef :type Emma%20Controller%20Object%20Reference))
  (bind _aschar_emma (Utilities|Casting|CastToChar_Emma (Pawn|GetControlledPawn PCRef)))
  (for _array_element (Variables|/Game/Gameplay/GeneralBPs/EmmaController.EmmaController_C|GetInventorySlots (Variables|/Game/Gameplay/GeneralBPs/Char_Emma.Char_Emma_C|GetController%20REF _aschar_emma))
    (CallFunction|ConstructonServer _array_element _aschar_emma))
  (for _array_element_2 (Variables|/Game/Gameplay/GeneralBPs/EmmaController.EmmaController_C|GetActionSlots (Variables|/Game/Gameplay/GeneralBPs/Char_Emma.Char_Emma_C|GetController%20REF _aschar_emma))
    _)
  (bind _completed (CallFunction|CheckifCompleted))
  (if _completed
    (Development|PrintString "Bridge built")))

(fn ConstructionScript)

(fn CheckifCompleted
  (for (_array_element _array_index) (Variables|Default|GetCurrentCompletion)
    (return (not (< (.Amount (Utilities|Struct|BreakS_Slots _array_element)) (.Amount (Utilities|Struct|BreakS_Slots (Utilities|Array|Get(acopy) (Variables|Default|GetRequiredItemsForCompletion) _array_index)))))))
  (return false))

(fn AddItemstoConstructions
  (params (AddedItem :type S%20Slots%20Structure) (PlayerReference :type Char%20Emma%20Object%20Reference))
  (bind (_item _amount) (Utilities|Struct|BreakS_Slots AddedItem))
  (bind (_datatable _rowname) (Utilities|Struct|BreakDataTableRowHandle _item))
  (LocalVariables|SetCharacterReference PlayerReference)
  (bind _returnvalue (Utilities|GetDataTableRow _datatable _rowname)
    (:then
      (bind (_array_element _array_index) (Utilities|Array|ForEachLoopwithBreak (Variables|Default|GetRequiredItemsForCompletion))
        (:LoopBody
          (bind _returnvalue_2 (Utilities|GetDataTableRow (.DataTable (Utilities|Struct|BreakDataTableRowHandle (.Item (Utilities|Struct|BreakS_Slots _array_element)))) (.RowName (Utilities|Struct|BreakDataTableRowHandle (.Item (Utilities|Struct|BreakS_Slots _array_element)))))
            (:then
              (if (Utilities|Enum|Equal(Enum) (.Name (Utilities|Struct|BreakS_Inventory _returnvalue_2)) (.Name (Utilities|Struct|BreakS_Inventory _returnvalue)))
                (bind _required (CallFunction|GetRequiredItemsOfType AddedItem))
                (if (<= _amount _required)
                  (Utilities|Array|SetArrayElem (Variables|Default|GetCurrentCompletion) _array_index (Utilities|Struct|MakeS_Slots (.Item (Utilities|Struct|BreakS_Slots (Utilities|Array|Get(acopy) (Variables|Default|GetCurrentCompletion) _array_index))) (+ (.Amount (Utilities|Struct|BreakS_Slots (Utilities|Array|Get(acopy) (Variables|Default|GetCurrentCompletion) _array_index))) _amount)))
                  (LocalVariables|SettmpSlot AddedItem)
                  (else
                    (Utilities|Array|SetArrayElem (Variables|Default|GetCurrentCompletion) _array_index (Utilities|Struct|MakeS_Slots (.Item (Utilities|Struct|BreakS_Slots (Utilities|Array|Get(acopy) (Variables|Default|GetCurrentCompletion) _array_index))) (+ (.Amount (Utilities|Struct|BreakS_Slots (Utilities|Array|Get(acopy) (Variables|Default|GetCurrentCompletion) _array_index))) _required)))
                    (LocalVariables|SettmpSlot (Utilities|Struct|MakeS_Slots (.Item (Utilities|Struct|BreakS_Slots AddedItem)) _required))))
                (for (_array_element_2 _array_index_2) (Variables|/Game/Gameplay/GeneralBPs/EmmaController.EmmaController_C|GetInventorySlots (Variables|/Game/Gameplay/GeneralBPs/Char_Emma.Char_Emma_C|GetController%20REF (LocalVariables|GetCharacterReference)))
                  (bind _returnvalue_3 (Utilities|GetDataTableRow (.DataTable (Utilities|Struct|BreakDataTableRowHandle (.Item (Utilities|Struct|BreakS_Slots _array_element_2)))) (.RowName (Utilities|Struct|BreakDataTableRowHandle (.Item (Utilities|Struct|BreakS_Slots _array_element_2)))))
                    (:then
                      (bind _returnvalue_4 (Utilities|GetDataTableRow (.DataTable (Utilities|Struct|BreakDataTableRowHandle (.Item (Utilities|Struct|BreakS_Slots (LocalVariables|GettmpSlot))))) (.RowName (Utilities|Struct|BreakDataTableRowHandle (.Item (Utilities|Struct|BreakS_Slots (LocalVariables|GettmpSlot))))))
                        (:then
                          (if (Utilities|Enum|Equal(Enum) (.Name (Utilities|Struct|BreakS_Inventory _returnvalue_4)) (.Name (Utilities|Struct|BreakS_Inventory _returnvalue_3)))
                            (if (== (- (.Amount (Utilities|Struct|BreakS_Slots _array_element_2)) (.Amount (Utilities|Struct|BreakS_Slots (LocalVariables|GettmpSlot)))) 0)
                              (Utilities|Array|SetArrayElem (Variables|/Game/Gameplay/GeneralBPs/EmmaController.EmmaController_C|GetInventorySlots (Variables|/Game/Gameplay/GeneralBPs/Char_Emma.Char_Emma_C|GetController%20REF (LocalVariables|GetCharacterReference))) _array_index_2 (Utilities|Struct|MakeS_Slots (Utilities|Struct|MakeDataTableRowHandle "/Game/Gameplay/Inventory/Data/InventoryData.InventoryData" "Empty")))
                              (else
                                (Utilities|Array|SetArrayElem (Variables|/Game/Gameplay/GeneralBPs/EmmaController.EmmaController_C|GetInventorySlots (Variables|/Game/Gameplay/GeneralBPs/Char_Emma.Char_Emma_C|GetController%20REF (LocalVariables|GetCharacterReference))) _array_index_2 (Utilities|Struct|MakeS_Slots (.Item (Utilities|Struct|BreakS_Slots _array_element_2)) (- (.Amount (Utilities|Struct|BreakS_Slots _array_element_2)) (.Amount (Utilities|Struct|BreakS_Slots (LocalVariables|GettmpSlot))))))))))))))
                (for (_array_element_3 _array_index_3) (Variables|/Game/Gameplay/GeneralBPs/EmmaController.EmmaController_C|GetActionSlots (Variables|/Game/Gameplay/GeneralBPs/Char_Emma.Char_Emma_C|GetController%20REF (LocalVariables|GetCharacterReference)))
                  (bind _returnvalue_5 (Utilities|GetDataTableRow (.DataTable (Utilities|Struct|BreakDataTableRowHandle (.Item (Utilities|Struct|BreakS_Slots _array_element_3)))) (.RowName (Utilities|Struct|BreakDataTableRowHandle (.Item (Utilities|Struct|BreakS_Slots _array_element_3)))))
                    (:then
                      (bind _returnvalue_6 (Utilities|GetDataTableRow (.DataTable (Utilities|Struct|BreakDataTableRowHandle (.Item (Utilities|Struct|BreakS_Slots (LocalVariables|GettmpSlot))))) (.RowName (Utilities|Struct|BreakDataTableRowHandle (.Item (Utilities|Struct|BreakS_Slots (LocalVariables|GettmpSlot))))))
                        (:then
                          (if (Utilities|Enum|Equal(Enum) (.Name (Utilities|Struct|BreakS_Inventory _returnvalue_6)) (.Name (Utilities|Struct|BreakS_Inventory _returnvalue_5)))
                            (if (== (- (.Amount (Utilities|Struct|BreakS_Slots _array_element_3)) (.Amount (Utilities|Struct|BreakS_Slots (LocalVariables|GettmpSlot)))) 0)
                              (Utilities|Array|SetArrayElem (Variables|/Game/Gameplay/GeneralBPs/EmmaController.EmmaController_C|GetActionSlots (Variables|/Game/Gameplay/GeneralBPs/Char_Emma.Char_Emma_C|GetController%20REF (LocalVariables|GetCharacterReference))) _array_index_3 (Utilities|Struct|MakeS_Slots (Utilities|Struct|MakeDataTableRowHandle "/Game/Gameplay/Inventory/Data/InventoryData.InventoryData" "Empty")))
                              (else
                                (Utilities|Array|SetArrayElem (Variables|/Game/Gameplay/GeneralBPs/EmmaController.EmmaController_C|GetActionSlots (Variables|/Game/Gameplay/GeneralBPs/Char_Emma.Char_Emma_C|GetController%20REF (LocalVariables|GetCharacterReference))) _array_index_3 (Utilities|Struct|MakeS_Slots (.Item (Utilities|Struct|BreakS_Slots _array_element_3)) (- (.Amount (Utilities|Struct|BreakS_Slots _array_element_3)) (.Amount (Utilities|Struct|BreakS_Slots (LocalVariables|GettmpSlot))))))))))))))
                (Default|RefreshHUD1 (Variables|/Game/Gameplay/GeneralBPs/Char_Emma.Char_Emma_C|GetController%20REF (LocalVariables|GetCharacterReference)))
                (Default|RemoveInv (Variables|/Game/Gameplay/GeneralBPs/Char_Emma.Char_Emma_C|GetController%20REF (LocalVariables|GetCharacterReference)))))))))))

(fn GetRequiredItemsOfType
  (params (Item :type S%20Slots%20Structure))
  (bind _item (Utilities|Struct|BreakS_Slots Item))
  (bind (_datatable _rowname) (Utilities|Struct|BreakDataTableRowHandle _item))
  (bind _returnvalue (Utilities|GetDataTableRow _datatable _rowname)
    (:then
      (for (_array_element _array_index) (Variables|Default|GetCurrentCompletion)
        (bind _returnvalue_2 (Utilities|GetDataTableRow (.DataTable (Utilities|Struct|BreakDataTableRowHandle (.Item (Utilities|Struct|BreakS_Slots _array_element)))) (.RowName (Utilities|Struct|BreakDataTableRowHandle (.Item (Utilities|Struct|BreakS_Slots _array_element)))))
          (:then
            (if (Utilities|Enum|Equal(Enum) (.Name (Utilities|Struct|BreakS_Inventory _returnvalue_2)) (.Name (Utilities|Struct|BreakS_Inventory _returnvalue)))
              (return (- (.Amount (Utilities|Struct|BreakS_Slots (Utilities|Array|Get(acopy) (Variables|Default|GetRequiredItemsForCompletion) _array_index))) (.Amount (Utilities|Struct|BreakS_Slots _array_element)))))))))))