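; Ore node that breaks apart in four stages, dropping Stone pickups and respawning through the game state.
; Each DestroyPart call applies radius damage to the current part, then the authority spawns a randomly offset pickup and advances the stage.
; The construction script pre-rolls each part's drop amount, and a helper rolls random XP.
; After the last part, the actor waits briefly, destroys itself and requests a timed respawn at its transform.
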(event Custom|DestroyPart
  (bind _part1 (Variables|Default|GetPart1))
  (bind _part2 (Variables|Default|GetPart2))
  (bind _part4 (Variables|Default|GetPart4))
  (bind _part3 (Variables|Default|GetPart3))
  (switch int (Variables|Default|GetcurrentPartForDestruction)
    (:0
      (Class|DestructibleComponent|ApplyRadiusDamage _part1 1e+01 (Transformation|GetWorldLocation _part1) 1e+01 0.01 false)
      (Networking|SwitchHasAuthority :!label _label
        (:Authority
          (bind _drops (CallFunction|GetDropsforCurrentPart))
          (Game|SpawnActorfromClass "/Game/Gameplay/PickUps/Pickup_Master.Pickup_Master_C" (Math|Transform|MakeTransform (+ (Transformation|GetActorLocation) (Math|Vector|MakeVector (Math|Random|RandomFloatinRange -1e+02 1e+02) (Math|Random|RandomFloatinRange -1e+02 1e+02) 1e+02)) "0, 0, 0" "1,1,1") "Undefined" 0 (Utilities|Struct|MakeS_Slots (Utilities|Struct|MakeDataTableRowHandle "/Game/Gameplay/Inventory/Data/InventoryData.InventoryData" "Stone") _drops) 0)
          (Math|Integer|IncrementInt (Variables|Default|GetcurrentPartForDestruction)))))
    (:1
      (Class|DestructibleComponent|ApplyRadiusDamage _part2 1e+01 (Transformation|GetWorldLocation _part2) 1e+01 0.01 false)
      (goto _label))
    (:2
      (Class|DestructibleComponent|ApplyRadiusDamage _part3 1e+01 (Transformation|GetWorldLocation _part3) 1e+01 0.01 false)
      (goto _label))
    (:3
      (Class|DestructibleComponent|ApplyRadiusDamage _part4 1e+01 (Transformation|GetWorldLocation _part4) 1e+01 0.01 false)
      (Utilities|FlowControl|Sequence
        (:then_0
          (goto _label))
        (:then_1
          (Utilities|FlowControl|Delay 3.0)
          (Actor|DestroyActor)
          (bind _ascode_name_protect_state (Utilities|Casting|CastToCODE_NAME_PROTECT_STATE (Game|GetGameState)))
          (Default|RespawnRecourceatLocationAfterTime _ascode_name_protect_state (Variables|Default|GetactorTransform) (Utilities|GetClass self)))))))

(fn ConstructionScript
  (for _index (range 0 3)
    (Utilities|Array|SetArrayElem (Variables|Default|GetDrops) _index (Math|Random|RandomIntegerinRange (Variables|Default|GetminDropsPerPart) (Variables|Default|GetmaxDropsPerPart)))))

(fn GetDropsforCurrentPart
  (return (Utilities|Array|Get(acopy) (Variables|Default|GetDrops) (Variables|Default|GetcurrentPartForDestruction))))

(fn GetRandomXP
  (return (Math|Random|RandomFloatinRange (Variables|Default|GetxpDropMin) (Variables|Default|GetxpDropMax))))