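; Choppable tree that topples when StartFalling is called, then turns into a Wood pickup.
; A delay loop steadily accelerates RotatingMovement, with rotation derived from the hit location relative to the trunk, until HitCollider overlaps the landscape.
; It then destroys itself, spawns a Pickup_Master with a random wood amount at its original location, and asks the game state to respawn a tree there after a random delay.
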(event Custom|StartFalling
  (params (HitLocation :type Vector))
  (bind _returnvalue (Utilities|Time|GetWorldDeltaSeconds))
  (bind _tree (Variables|Default|GetTree))
  (bind _returnvalue_2 (Transformation|GetWorldLocation _tree))
  (bind _returnvalue_3 (- HitLocation _returnvalue_2))
  (bind _returnvalue_4 (Class|KismetMathLibrary|VectorNormal2D _returnvalue_3 0.0001))
  (Variables|Default|Setfalling true)
  (Variables|Default|SetFallDirection (Math|Vector2D|MakeVector2D (.x _returnvalue_4) (.y _returnvalue_4)))
  (if (> (Utilities|Array|Length (Collision|GetOverlappingActors (Variables|Default|GetHitCollider) "/Script/Landscape.Landscape" :!class /Script/Engine.PrimitiveComponent)) 0) :!label _label
    (Variables|/Script/Engine.RotatingMovementComponent|SetRotationRate (Variables|Default|GetRotatingMovement) (Math|Rotator|MakeRotator 0.0 0.0 0.0))
    (Actor|DestroyActor)
    (Game|SpawnActorfromClass "/Game/Gameplay/PickUps/Pickup_Master.Pickup_Master_C" (Math|Transform|MakeTransform (Variables|Default|GetactorLocation) "0, 0, 0" "1,1,1") "Undefined" 0 (Utilities|Struct|MakeS_Slots (Utilities|Struct|MakeDataTableRowHandle "/Game/Gameplay/Inventory/Data/InventoryData.InventoryData" "Wood") (Math|Random|RandomIntegerinRange (Variables|Default|GetminDropPieces) (Variables|Default|GetmaxDropPieces))) 0)
    (bind _ascode_name_protect_state (Utilities|Casting|CastToCODE_NAME_PROTECT_STATE (Game|GetGameState)))
    (Default|RespawnTreeatLocationAfterTime _ascode_name_protect_state (Variables|Default|GetactorLocation) (Math|Random|RandomIntegerinRange 50 60))
    (else
      (Utilities|FlowControl|Delay _returnvalue)
      (bind _output_get (Variables|Default|Setspeed (+ (Variables|Default|Getspeed) (* _returnvalue (Variables|Default|Getspeed)))))
      (Variables|/Script/Engine.RotatingMovementComponent|SetRotationRate (Variables|Default|GetRotatingMovement) (Math|Rotator|MakeRotator (.x (* (Variables|Default|GetFallDirection) _output_get)) (.y (* (Variables|Default|GetFallDirection) _output_get)) 0.0))
      (goto _label))))

(event EventBeginPlay
  (Variables|/Script/Engine.RotatingMovementComponent|SetRotationRate (Variables|Default|GetRotatingMovement) (Math|Rotator|MakeRotator 0.0 0.0 0.0))
  (Variables|Default|SetactorLocation (Transformation|GetActorLocation)))

(fn ConstructionScript)