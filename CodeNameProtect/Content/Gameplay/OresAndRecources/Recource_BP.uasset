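; Harvestable resource node that breaks apart in four stages, each yielding a drop amount and random XP.
; The construction script pre-rolls each part's drop count.
; Each DestroyPart event fractures the next part with tiny radius damage, announces the drop and grants XP through Char_Emma, destroying the actor shortly after the last.
; Separate per-part functions flag a part destroyed, grant XP and return its drop count.
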(event Custom|DestroyPart
  (bind _part1 (Variables|Default|GetPart1))
  (bind _part2 (Variables|Default|GetPart2))
  (bind _part3 (Variables|Default|GetPart3))
  (bind _part4 (Variables|Default|GetPart4))
  (switch int (Variables|Default|GetcurrentPartForDestruction)
    (:0
      (Class|DestructibleComponent|ApplyRadiusDamage _part1 1e+01 (Transformation|GetWorldLocation _part1) 1e+01 0.01 false)
      (bind _aschar_emma (Utilities|Casting|CastToChar_Emma (Pawn|GetControlledPawn (Game|GetPlayerController 0)) :!label _label))
      (Default|AddAnnouncement (Variables|/Game/Gameplay/GeneralBPs/Char_Emma.Char_Emma_C|GetCollectedItemWidgetReference _aschar_emma) (Utilities|Array|Get(acopy) (Variables|Default|GetDrops) (Variables|Default|GetcurrentPartForDestruction)) (Variables|Default|GetrecourceName))
      (Default|AddExp (Variables|/Game/Gameplay/GeneralBPs/Char_Emma.Char_Emma_C|GetLevelingSystem _aschar_emma) (Math|Random|RandomFloatinRange (Variables|Default|GetxpDropMin) (Variables|Default|GetxpDropMax)))
      (Math|Integer|IncrementInt (Variables|Default|GetcurrentPartForDestruction)))
    (:1
      (Class|DestructibleComponent|ApplyRadiusDamage _part2 1e+01 (Transformation|GetWorldLocation _part2) 1e+01 0.01 false)
      (goto _label))
    (:2
      (Class|DestructibleComponent|ApplyRadiusDamage _part3 1e+01 (Transformation|GetWorldLocation _part3) 1e+01 0.01 false)
      (goto _label))
    (:3
      (Class|DestructibleComponent|ApplyRadiusDamage _part4 1e+01 (Transformation|GetWorldLocation _part4) 1e+01 0.01 false)
      (Utilities|FlowControl|Sequence
        (:then_0
          (goto _label))
        (:then_1
          (Utilities|FlowControl|Delay 3.0)
          (Actor|DestroyActor))))))

(fn ConstructionScript
  (for _index (range 0 3)
    (Utilities|Array|SetArrayElem (Variables|Default|GetDrops) _index (Math|Random|RandomIntegerinRange (Variables|Default|GetminDropsPerPart) (Variables|Default|GetmaxDropsPerPart)))))

(fn DestroyPart1
  (Utilities|Array|SetArrayElem (Variables|Default|GetpartsDestroyed) 0 true)
  (CallFunction|GiveXPtoPlayer)
  (return (Utilities|Array|Get(acopy) (Variables|Default|GetDrops))))

(fn DestroyPart2
  (Utilities|Array|SetArrayElem (Variables|Default|GetpartsDestroyed) 1 true)
  (CallFunction|GiveXPtoPlayer)
  (return (Utilities|Array|Get(acopy) (Variables|Default|GetDrops) 1)))

(fn DestroyPart3
  (Utilities|Array|SetArrayElem (Variables|Default|GetpartsDestroyed) 2 true)
  (CallFunction|GiveXPtoPlayer)
  (return (Utilities|Array|Get(acopy) (Variables|Default|GetDrops) 2)))

(fn DestroyPart4
  (Utilities|Array|SetArrayElem (Variables|Default|GetpartsDestroyed) 3 true)
  (CallFunction|GiveXPtoPlayer)
  (return (Utilities|Array|Get(acopy) (Variables|Default|GetDrops) 3)))

(fn GiveXPtoPlayer
  (bind _aschar_emma (Utilities|Casting|CastToChar_Emma (Game|GetPlayerCharacter 0)))
  (Default|AddExp (Variables|/Game/Gameplay/GeneralBPs/Char_Emma.Char_Emma_C|GetLevelingSystem _aschar_emma) (Math|Random|RandomFloatinRange (Variables|Default|GetxpDropMin) (Variables|Default|GetxpDropMax))))