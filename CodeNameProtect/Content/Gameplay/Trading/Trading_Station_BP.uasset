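; Trading station actor that sells one configured item for materials when Char_Emma interacts, showing the item's name and amount on its trader widget.
; DoPurchase reads the data-table price, then requires enough of each material in a single slot plus an empty slot.
; It deducts from inventory slots, though the action-bar pass compares against the inventory loop element, not the price.
; The controller then stacks or slots the item and refreshes the HUD.
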(event EventBeginPlay
  (Utilities|FlowControl|Delay 0.2)
  (bind _output_get (Variables|Default|SetReceivingItem (Utilities|Struct|MakeS_Slots (.Item (Utilities|Struct|BreakS_Slots (Variables|Default|GetReceivingItem))) (Variables|Default|Getamount))))
  (bind _returnvalue (Utilities|GetDataTableRow (.DataTable (Utilities|Struct|BreakDataTableRowHandle (.Item (Utilities|Struct|BreakS_Slots _output_get)))) (.RowName (Utilities|Struct|BreakDataTableRowHandle (.Item (Utilities|Struct|BreakS_Slots _output_get)))))
    (:then
      (Default|ChangeInfo (Variables|Default|GetTraderWidget) (.Name (Utilities|Struct|BreakS_Inventory _returnvalue)) (Variables|Default|Getamount)))))

(event EventInteract
  (params (PCRef :type Emma%20Controller%20Object%20Reference))
  (bind _aschar_emma (Utilities|Casting|CastToChar_Emma (Pawn|GetControlledPawn PCRef)))
  (Variables|Default|SetPlayerReference _aschar_emma)
  (CallFunction|DoPurchase (Variables|Default|GetReceivingItem)))

(fn ConstructionScript)

(fn GetRequiredMaterialsforPurchase
  (params (ItemToPurchase :type S%20Slots%20Structure))
  (bind _item (Utilities|Struct|BreakS_Slots ItemToPurchase))
  (bind (_datatable _rowname) (Utilities|Struct|BreakDataTableRowHandle _item))
  (bind _returnvalue (Utilities|GetDataTableRow _datatable _rowname)
    (:then
      (return (.PriceToObtain (Utilities|Struct|BreakS_Inventory _returnvalue))))))

(fn HasPlayerEnoughMaterialsforPurchase
  (params (ItemToPurchase :type S%20Slots%20Structure))
  (bind _playerreference (Variables|Default|GetPlayerReference))
  (bind _tmpinventoryslots (LocalVariables|GettmpInventorySlots))
  (bind _controller_ref (Variables|/Game/Gameplay/GeneralBPs/Char_Emma.Char_Emma_C|GetController%20REF _playerreference))
  (bind _materials (CallFunction|GetRequiredMaterialsforPurchase ItemToPurchase))
  (for _array_element _materials
    (LocalVariables|SetfoundItem false)
    (Utilities|Array|AppendArray _tmpinventoryslots (Variables|/Game/Gameplay/GeneralBPs/EmmaController.EmmaController_C|GetInventorySlots _controller_ref))
    (Utilities|Array|AppendArray _tmpinventoryslots (Variables|/Game/Gameplay/GeneralBPs/EmmaController.EmmaController_C|GetActionSlots _controller_ref))
    (for _array_element_2 (LocalVariables|GettmpInventorySlots)
      (bind _returnvalue (Utilities|GetDataTableRow (.DataTable (Utilities|Struct|BreakDataTableRowHandle (.Item (Utilities|Struct|BreakS_Slots _array_element_2)))) (.RowName (Utilities|Struct|BreakDataTableRowHandle (.Item (Utilities|Struct|BreakS_Slots _array_element_2)))))
        (:then
          (bind _returnvalue_2 (Utilities|GetDataTableRow (.DataTable (Utilities|Struct|BreakDataTableRowHandle (.Item (Utilities|Struct|BreakS_Slots _array_element)))) (.RowName (Utilities|Struct|BreakDataTableRowHandle (.Item (Utilities|Struct|BreakS_Slots _array_element)))))
            (:then
              (if (Utilities|Enum|Equal(Enum) (.Name (Utilities|Struct|BreakS_Inventory _returnvalue)) (.Name (Utilities|Struct|BreakS_Inventory _returnvalue_2)))
                (if (>= (.Amount (Utilities|Struct|BreakS_Slots _array_element_2)) (.Amount (Utilities|Struct|BreakS_Slots _array_element)))
                  (LocalVariables|SetfoundItem true))))))))
    (if (not (LocalVariables|GetfoundItem))
      (return false)))
  (return true))

(fn DoPurchase
  (params (ItemToPurchase :type S%20Slots%20Structure))
  (bind _item (Utilities|Struct|BreakS_Slots ItemToPurchase))
  (bind _playerreference (Variables|Default|GetPlayerReference))
  (bind _playerreference_2 (Variables|Default|GetPlayerReference))
  (bind (_datatable _rowname) (Utilities|Struct|BreakDataTableRowHandle _item))
  (bind _controller_ref (Variables|/Game/Gameplay/GeneralBPs/Char_Emma.Char_Emma_C|GetController%20REF _playerreference))
  (bind _controller_ref_2 (Variables|/Game/Gameplay/GeneralBPs/Char_Emma.Char_Emma_C|GetController%20REF _playerreference_2))
  (bind _inventoryslots (Variables|/Game/Gameplay/GeneralBPs/EmmaController.EmmaController_C|GetInventorySlots _controller_ref_2))
  (bind _actionslots (Variables|/Game/Gameplay/GeneralBPs/EmmaController.EmmaController_C|GetActionSlots _controller_ref_2))
  (bind _hasenoughitems (CallFunction|HasPlayerEnoughMaterialsforPurchase ItemToPurchase))
  (bind _hasspace (CallFunction|HasPlayerEnoughSpaceinInventory))
  (if (and _hasenoughitems _hasspace)
    (bind _materials (CallFunction|GetRequiredMaterialsforPurchase ItemToPurchase))
    (for _array_element _materials
      ;[1 1 1] Check inventory and action bar for required items
      (for (_array_element_2 _array_index) _inventoryslots
        (bind _returnvalue (Utilities|GetDataTableRow (.DataTable (Utilities|Struct|BreakDataTableRowHandle (.Item (Utilities|Struct|BreakS_Slots _array_element_2)))) (.RowName (Utilities|Struct|BreakDataTableRowHandle (.Item (Utilities|Struct|BreakS_Slots _array_element_2)))))
          (:then
            (bind _returnvalue_2 (Utilities|GetDataTableRow (.DataTable (Utilities|Struct|BreakDataTableRowHandle (.Item (Utilities|Struct|BreakS_Slots _array_element)))) (.RowName (Utilities|Struct|BreakDataTableRowHandle (.Item (Utilities|Struct|BreakS_Slots _array_element)))))
              (:then
                (if (Utilities|Enum|Equal(Enum) (.Name (Utilities|Struct|BreakS_Inventory _returnvalue_2)) (.Name (Utilities|Struct|BreakS_Inventory _returnvalue)))
                  (if (== (- (.Amount (Utilities|Struct|BreakS_Slots _array_element_2)) (.Amount (Utilities|Struct|BreakS_Slots _array_element))) 0)
                    (Utilities|Array|SetArrayElem _inventoryslots _array_index (Utilities|Struct|MakeS_Slots (Utilities|Struct|MakeDataTableRowHandle "/Game/Gameplay/Inventory/Data/InventoryData.InventoryData" "Empty")))
                    (else
                      (Utilities|Array|SetArrayElem _inventoryslots _array_index (Utilities|Struct|MakeS_Slots (.Item (Utilities|Struct|BreakS_Slots _array_element_2)) (- (.Amount (Utilities|Struct|BreakS_Slots _array_element_2)) (.Amount (Utilities|Struct|BreakS_Slots _array_element)))))))))))))
      (for (_array_element_3 _array_index_2) _actionslots
        (bind _returnvalue_3 (Utilities|GetDataTableRow (.DataTable (Utilities|Struct|BreakDataTableRowHandle (.Item (Utilities|Struct|BreakS_Slots _array_element_3)))) (.RowName (Utilities|Struct|BreakDataTableRowHandle (.Item (Utilities|Struct|BreakS_Slots _array_element_3)))))
          (:then
            (bind _returnvalue_4 (Utilities|GetDataTableRow (.DataTable (Utilities|Struct|BreakDataTableRowHandle (.Item (Utilities|Struct|BreakS_Slots _array_element_2)))) (.RowName (Utilities|Struct|BreakDataTableRowHandle (.Item (Utilities|Struct|BreakS_Slots _array_element_2)))))
              (:then
                (if (Utilities|Enum|Equal(Enum) (.Name (Utilities|Struct|BreakS_Inventory _returnvalue_4)) (.Name (Utilities|Struct|BreakS_Inventory _returnvalue_3)))
                  (if (== (- (.Amount (Utilities|Struct|BreakS_Slots _array_element_3)) (.Amount (Utilities|Struct|BreakS_Slots _array_element_2))) 0)
                    (Utilities|Array|SetArrayElem _actionslots _array_index_2 (Utilities|Struct|MakeS_Slots (Utilities|Struct|MakeDataTableRowHandle "/Game/Gameplay/Inventory/Data/InventoryData.InventoryData" "Empty")))
                    (else
                      (Utilities|Array|SetArrayElem _actionslots _array_index_2 (Utilities|Struct|MakeS_Slots (.Item (Utilities|Struct|BreakS_Slots _array_element_3)) (- (.Amount (Utilities|Struct|BreakS_Slots _array_element_3)) (.Amount (Utilities|Struct|BreakS_Slots _array_element_2))))))))))))))
    (bind _returnvalue_5 (Utilities|GetDataTableRow _datatable _rowname)
      (:then
        (if (.CanStack? (Utilities|Struct|BreakS_Inventory _returnvalue_5))
          (bind (_array_index_3 _success) (Default|HasItemAlready? _controller_ref ItemToPurchase))
          (if _success
            (Default|PUAdd _controller_ref _array_index_3 ItemToPurchase)
            (Default|RefreshHUD1 _controller_ref :!label _label)
            (Default|RemoveInv _controller_ref)
            (return true)
            (else
              (bind (_array_index_4 _success_2) (Default|GetEmptySlot _controller_ref :!label _label_2))
              (if _success_2
                (Default|PUSlot _controller_ref _array_index_4 ItemToPurchase)
                (goto _label))))
          (else
            (goto _label_2)))))
    (else
      (return false))))

(fn HasPlayerEnoughSpaceinInventory
  (bind _playerreference (Variables|Default|GetPlayerReference))
  (bind _tmpinventoryslots (LocalVariables|GettmpInventorySlots))
  (bind _controller_ref (Variables|/Game/Gameplay/GeneralBPs/Char_Emma.Char_Emma_C|GetController%20REF _playerreference))
  (Utilities|Array|AppendArray _tmpinventoryslots (Variables|/Game/Gameplay/GeneralBPs/EmmaController.EmmaController_C|GetInventorySlots _controller_ref))
  (Utilities|Array|AppendArray _tmpinventoryslots (Variables|/Game/Gameplay/GeneralBPs/EmmaController.EmmaController_C|GetActionSlots _controller_ref))
  (for _array_element (LocalVariables|GettmpInventorySlots)
    (bind _returnvalue (Utilities|GetDataTableRow (.DataTable (Utilities|Struct|BreakDataTableRowHandle (.Item (Utilities|Struct|BreakS_Slots _array_element)))) (.RowName (Utilities|Struct|BreakDataTableRowHandle (.Item (Utilities|Struct|BreakS_Slots _array_element)))))
      (:then
        (if (Utilities|Enum|Equal(Enum) (.Name (Utilities|Struct|BreakS_Inventory _returnvalue)) "Empty")
          (return true)))))
  (return false))