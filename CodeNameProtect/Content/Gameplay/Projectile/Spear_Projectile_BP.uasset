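; Spear projectile Blueprint that flies via a ProjectileMovement component and sticks into NPCs it hits.
; While flying, Tick applies a small fixed world pitch rotation to the spear each frame, independent of delta time, to tip it downward.
; When the capsule overlaps an NPC_BASE_CLASS actor, it stops movement, ends the flight rotation and attaches to the NPC's mesh using KeepRelative rules.
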(event OnComponentBeginOverlap(Capsule)
  (params (OverlappedComponent :type Primitive%20Component%20Object%20Reference) (OtherActor :type Actor%20Object%20Reference) (OtherComp :type Primitive%20Component%20Object%20Reference) (OtherBodyIndex :type Integer) (bFromSweep :type Boolean) (SweepResult :type Hit%20Result%20Structure%20%28by%20ref%29))
  (bind _asnpc_base_class (Utilities|Casting|CastToNPC_BASE_CLASS OtherActor))
  (Components|Movement|StopMovementImmediately (Variables|Default|GetProjectileMovement))
  (Variables|Default|SetisFlying false)
  (Transformation|AttachComponentToComponent self (Variables|/Script/Engine.Character|GetMesh _asnpc_base_class) "None" "KeepRelative" "KeepRelative" "KeepRelative" true))

(event EventTick
  (params (DeltaSeconds :type Float%20%28single-precision%29))
  (if (Variables|Default|GetisFlying)
    (Transformation|AddWorldRotation (Variables|Default|GetSpear) (Math|Rotator|MakeRotator 0.0 -0.5 0.0) true false)))

(fn ConstructionScript)