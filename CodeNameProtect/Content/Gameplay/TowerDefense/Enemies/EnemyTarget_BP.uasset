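; Tower defense goal actor that ends the game when too many standard enemies occupy it at once.
; Server-only overlap events on EnemyCollider keep a live count of StandardEnemy_BP actors inside, rising on entry and falling on exit.
; When the count reaches EnemiesUntilGameOver, it finds a Char_Emma and calls NewMapOnServer on it.
; A disconnected session-search chain that compares extra settings remains in the graph and never runs.
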(event OnComponentBeginOverlap(EnemyCollider)
  (params (OverlappedComponent :type Primitive%20Component%20Object%20Reference) (OtherActor :type Actor%20Object%20Reference) (OtherComp :type Primitive%20Component%20Object%20Reference) (OtherBodyIndex :type Integer) (bFromSweep :type Boolean) (SweepResult :type Hit%20Result%20Structure%20%28by%20ref%29))
  (Networking|SwitchHasAuthority
    (:Authority
      (Utilities|Casting|CastToStandardEnemy_BP OtherActor)
      (Math|Integer|IncrementInt (Variables|Default|GetenemiesInTarget)
        (:%20%20
          (if (>= (Variables|Default|GetenemiesInTarget) (Variables|Default|GetenemiesUntilGameOver))
            (bind _returnvalue (Actor|GetActorOfClass "/Game/Gameplay/GeneralBPs/Char_Emma.Char_Emma_C"))
            (Default|NewMaponServer _returnvalue)))))))

(event OnComponentEndOverlap(EnemyCollider)
  (params (OverlappedComponent :type Primitive%20Component%20Object%20Reference) (OtherActor :type Actor%20Object%20Reference) (OtherComp :type Primitive%20Component%20Object%20Reference) (OtherBodyIndex :type Integer))
  (Networking|SwitchHasAuthority
    (:Authority
      (Utilities|Casting|CastToStandardEnemy_BP OtherActor)
      (Math|Integer|DecrementInt (Variables|Default|GetenemiesInTarget)))))

(fn ConstructionScript)