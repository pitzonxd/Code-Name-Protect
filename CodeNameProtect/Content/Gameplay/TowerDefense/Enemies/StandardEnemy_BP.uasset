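; StandardEnemy_BP is a tower defense enemy that tracks its health and dies when it runs out.
; The construction script sets current health to max health, and any damage received subtracts from it.
; At zero or below, it casts the player character to Char_Emma, removes itself from that character's grid reference, and destroys itself.
; If the cast fails, the enemy is not destroyed.
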(event Game|Damage|EventAnyDamage
  (params (Damage :type Float%20%28single-precision%29) (DamageType :type Damage%20Type%20Object%20Reference) (InstigatedBy :type Controller%20Object%20Reference) (DamageCauser :type Actor%20Object%20Reference))
  (Variables|Default|SetcurrentHealth (- (Variables|Default|GetcurrentHealth) Damage))
  (if (<= (Variables|Default|GetcurrentHealth) 0.0)
    (bind _aschar_emma (Utilities|Casting|CastToChar_Emma (Game|GetPlayerCharacter 0)))
    (Default|RemoveDeadEnemy (Variables|/Game/Gameplay/GeneralBPs/Char_Emma.Char_Emma_C|GetGridReference _aschar_emma) self)
    (Actor|DestroyActor)))

(fn ConstructionScript
  (Variables|Default|SetcurrentHealth (Variables|Default|GetmaxHealth)))