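; Tower defense grid actor that spawns a tile field and manages the enemy list.
; Char_Emma entering or leaving HitBox makes Tick start a delayed ripple from the character's last grid position, lighting or dimming tiles through a C++ RecursiveSpawning component.
; Pressing Z spawns behavior-tree enemies at random points inside CharacterHitbox but outside the grid, using rejection sampling.
; It also removes dead enemies and finds a tower's closest enemy within damage radius.
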(event OnComponentEndOverlap(HitBox)
  (params (OverlappedComponent :type Primitive%20Component%20Object%20Reference) (OtherActor :type Actor%20Object%20Reference) (OtherComp :type Primitive%20Component%20Object%20Reference) (OtherBodyIndex :type Integer))
  (if (Variables|Default|GetLight)
    (if (== (Utilities|Array|Length (Collision|GetOverlappingActors (Variables|Default|GetHitBox) "/Game/Gameplay/GeneralBPs/Char_Emma.Char_Emma_C" :!class /Script/Engine.PrimitiveComponent)) 0)
      (Utilities|Casting|CastToChar_Emma OtherActor)
      (Variables|Default|SetplayerLeft true))))

(event OnComponentBeginOverlap(HitBox)
  (params (OverlappedComponent :type Primitive%20Component%20Object%20Reference) (OtherActor :type Actor%20Object%20Reference) (OtherComp :type Primitive%20Component%20Object%20Reference) (OtherBodyIndex :type Integer) (bFromSweep :type Boolean) (SweepResult :type Hit%20Result%20Structure%20%28by%20ref%29))
  (if (not (Variables|Default|GetLight))
    (if (== (Utilities|Array|Length (Collision|GetOverlappingActors (Variables|Default|GetHitBox) "/Game/Gameplay/GeneralBPs/Char_Emma.Char_Emma_C" :!class /Script/Engine.PrimitiveComponent)) 1)
      (Utilities|Casting|CastToChar_Emma OtherActor)
      (Variables|Default|SetplayerCame true))))

(event Custom|RemoveDeadEnemy
  (params (NewParam :type Standard%20Enemy%20BP%20Object%20Reference))
  ;[1 1 1] Remove dead enemy (Called from StandartEemyBP)
  (Actor|DestroyActor NewParam)
  (Utilities|Array|RemoveItem (Variables|Default|GetAllEnemies) NewParam))

(event Custom|LightAtPosition
  (params (Position :type Vector) (LightUp :type Boolean))
  (bind _returnvalue (Class|RecursiveSpawningCPP|TranslatePositiontoRowsandCols (Variables|Default|GetRecursiveSpawningRef) (.x Position) (.y Position) (.z Position)))
  (if LightUp
    (Default|LightUp (Utilities|Array|Get(acopy) (Variables|Default|GetTilesArray) (+ (* (.x _returnvalue) (Variables|Default|Getcols)) (.y _returnvalue))))
    (else
      (Default|LightDown (Utilities|Array|Get(acopy) (Variables|Default|GetTilesArray) (+ (* (.x _returnvalue) (Variables|Default|Getcols)) (.y _returnvalue)))))))

(event EventTick
  (params (DeltaSeconds :type Float%20%28single-precision%29))
  (bind _hitbox (Variables|Default|GetHitBox))
  (bind _hitbox_2 (Variables|Default|GetHitBox))
  (bind _overlappingactors (Collision|GetOverlappingActors _hitbox "/Game/Gameplay/GeneralBPs/Char_Emma.Char_Emma_C" :!class /Script/Engine.PrimitiveComponent))
  (bind _overlappingactors_2 (Collision|GetOverlappingActors _hitbox_2 "/Game/Gameplay/GeneralBPs/Char_Emma.Char_Emma_C" :!class /Script/Engine.PrimitiveComponent))
  (if (> (Utilities|Array|Length _overlappingactors_2) 0)
    (bind _aschar_emma (Utilities|Casting|CastToChar_Emma (Utilities|Array|Get(acopy) _overlappingactors_2)))
    (bind _char_location (Default|GetCharacterPosition _aschar_emma))
    (bind _returnvalue (Class|RecursiveSpawningCPP|IsValidPosition (Variables|Default|GetRecursiveSpawningRef) _char_location))
    (if _returnvalue
      (Variables|Default|SetcharacterLocationInGrid _char_location)
      (if (Variables|Default|GetplayerCame) :!label _label
        (if (== (Utilities|Array|Length _overlappingactors) 1)
          (bind _aschar_emma_2 (Utilities|Casting|CastToChar_Emma (Utilities|Array|Get(acopy) _overlappingactors)))
          (bind _char_location_2 (Default|GetCharacterPosition _aschar_emma_2))
          (bind _returnvalue_2 (Class|RecursiveSpawningCPP|IsValidPosition (Variables|Default|GetRecursiveSpawningRef) _char_location_2))
          (if _returnvalue_2
            (Variables|Default|SetcharacterLocationInGrid _char_location_2)
            (if (Variables|Default|GetplayerCame)
              (Variables|Default|SetplayerCame false)
              (bind _returnvalue_3 (Class|RecursiveSpawningCPP|Stepon (Variables|Default|GetRecursiveSpawningRef) (Variables|Default|GetcharacterLocationInGrid)))
              (if _returnvalue_3
                ;[1 1 1] Light up everything
                (CallFunction|LightatPosition (Variables|Default|GetcharacterLocationInGrid) true)
                (Utilities|FlowControl|Delay 0.05 :!label _label_2)
                (bind _returnvalue_4 (Class|RecursiveSpawningCPP|UncoverTick (Variables|Default|GetRecursiveSpawningRef)))
                (if (== (Utilities|Array|Length _returnvalue_4) 0)
                  (Variables|Default|SetLight true)
                  (Class|RecursiveSpawningCPP|Reset (Variables|Default|GetRecursiveSpawningRef))
                  (else
                    (for _array_element _returnvalue_4
                      (CallFunction|LightatPosition _array_element true)
                      (goto _label_2)))))
              (else
                (if (Variables|Default|GetplayerLeft) :!label _label_3
                  (Variables|Default|SetplayerLeft false)
                  (bind _returnvalue_5 (Class|RecursiveSpawningCPP|Stepon (Variables|Default|GetRecursiveSpawningRef) (Variables|Default|GetcharacterLocationInGrid)))
                  (if _returnvalue_5
                    ;[1 1 1] Light up everything
                    (CallFunction|LightatPosition (Variables|Default|GetcharacterLocationInGrid) false)
                    (Utilities|FlowControl|Delay 0.05 :!label _label_4)
                    (bind _returnvalue_6 (Class|RecursiveSpawningCPP|UncoverTick (Variables|Default|GetRecursiveSpawningRef)))
                    (if (== (Utilities|Array|Length _returnvalue_6) 0)
                      (Variables|Default|SetLight false)
                      (Class|RecursiveSpawningCPP|Reset (Variables|Default|GetRecursiveSpawningRef))
                      (else
                        (for _array_element_2 _returnvalue_6
                          (CallFunction|LightatPosition _array_element_2 false)
                          (goto _label_4))))))))))
        (else
          (goto _label_3))))
    (else
      (goto _label))))

(event EventBeginPlay
  (bind _realorigin (Variables|Default|GetRealOrigin))
  (bind _returnvalue (AddComponent|AddRecursiveSpawningCPP))
  (bind _output_get (Variables|Default|SetRecursiveSpawningRef _returnvalue))
  (Class|RecursiveSpawningCPP|InitializeVariables _output_get (Variables|Default|GetRealOrigin) (Variables|Default|Getrows) (Variables|Default|Getcols))
  (for _index (range 0 (- (Variables|Default|Getrows) 1))
    (for _index_2 (range 0 (- (Variables|Default|Getcols) 1))
      (bind _returnvalue_2 (Game|SpawnActorfromClass "/Game/Gameplay/TowerDefense/Tile_BP.Tile_BP_C" (Math|Transform|MakeTransform (Math|Vector|MakeVector (+ (.x _realorigin) (* _index 2e+02)) (+ (.y _realorigin) (* _index_2 2e+02)) (.z _realorigin)) "0, 0, 0" "1,1,1") "Undefined" 0 0))
      (Utilities|Array|SetArrayElem (Variables|Default|GetTilesArray) (+ (* _index (Variables|Default|Getcols)) _index_2) _returnvalue_2 true))))

(event Input|KeyboardEvents|Z
  (params (Key :type Key%20Structure :default "None"))
  (bind _characterhitbox (Variables|Default|GetCharacterHitbox))
  (bind _hitbox (Variables|Default|GetHitBox))
  (bind (_origin _boxextent) (Collision|GetComponentBounds _hitbox))
  (bind (_origin_2 _boxextent_2) (Collision|GetComponentBounds _characterhitbox))
  (:Pressed
    (while (< (Variables|Default|GetspawnedEnemies) (Variables|Default|GetEnemiesToSpawn))
      (Variables|Default|SetTargetSpawnLocation (Math|Vector|MakeVector (+ (.x _origin_2) (* (.x _boxextent_2) (Math|Random|RandomFloatinRange -0.95 0.95))) (+ (.y _origin_2) (* (.y _boxextent_2) (Math|Random|RandomFloatinRange -0.95 0.95))) (.z (.Origin (Collision|GetComponentBounds (Variables|Default|GetCharacterHitbox))))))
      (if (not (and (and (< (.x (Variables|Default|GetTargetSpawnLocation)) (+ (.x _origin) (.x _boxextent))) (> (.x (Variables|Default|GetTargetSpawnLocation)) (- (.x _origin) (.x _boxextent)))) (and (< (.y (Variables|Default|GetTargetSpawnLocation)) (+ (.y _origin) (.y _boxextent))) (> (.y (Variables|Default|GetTargetSpawnLocation)) (- (.y _origin) (.y _boxextent))))))
        (bind _returnvalue (AI|SpawnAIFromClass "/Game/Gameplay/TowerDefense/Enemies/StandardEnemy_BP.StandardEnemy_BP_C" "/Game/Gameplay/TowerDefense/Enemies/Enemy_BT.Enemy_BT" (Variables|Default|GetTargetSpawnLocation) "0, 0, 0" false 0))
        (bind _asstandard_enemy_bp (Utilities|Casting|CastToStandardEnemy_BP _returnvalue))
        (Utilities|Array|Add (Variables|Default|GetAllEnemies) _asstandard_enemy_bp)
        (Math|Integer|IncrementInt (Variables|Default|GetspawnedEnemies))))
    (Variables|Default|SetspawnedEnemies 0)))

(fn ConstructionScript
  (Components|Box|SetBoxExtent (Variables|Default|GetHitBox) (Math|Vector|MakeVector (* (Variables|Default|Getrows) 1e+02) (* (Variables|Default|Getcols) 1e+02) 2e+02) true)
  (|CalculateOrigin))

(fn GetClosestEnemytoTower
  (params (Tower :type Target%20BP%20Object%20Reference) (damageradius :type Float%20%28single-precision%29))
  (bind _allenemies (Variables|Default|GetAllEnemies))
  (LocalVariables|SettmpTower Tower)
  (LocalVariables|SetdamageRadiusTmp damageradius)
  (if (== (Utilities|Array|Length (Variables|Default|GetAllEnemies)) 0)
    (return 0)
    (else
      (LocalVariables|SetClosestEnemy (Utilities|Array|Get(acopy) _allenemies))
      (for _index (range 1 (- (Utilities|Array|Length _allenemies) 1))
        (if (< (Transformation|GetDistanceTo (LocalVariables|GettmpTower) (Utilities|Array|Get(acopy) (Variables|Default|GetAllEnemies) _index)) (Transformation|GetDistanceTo (LocalVariables|GettmpTower) (LocalVariables|GetClosestEnemy)))
          (LocalVariables|SetClosestEnemy (Utilities|Array|Get(acopy) (Variables|Default|GetAllEnemies) _index))))
      (if (<= (Transformation|GetDistanceTo (LocalVariables|GetClosestEnemy) (LocalVariables|GettmpTower)) (LocalVariables|GetdamageRadiusTmp))
        (return (LocalVariables|GetClosestEnemy))
        (else
          (return 0))))))

(fn GetOffset
  (bind _returnvalue (Class|RecursiveSpawningCPP|CalculateOffset (Variables|Default|GetRecursiveSpawningRef) (Transformation|GetActorLocation)))
  (return _returnvalue))

(fn PositionValid
  (params (Poisition :type Vector))
  (bind _returnvalue (Class|RecursiveSpawningCPP|IsValidPosition (Variables|Default|GetRecursiveSpawningRef) Poisition))
  (return _returnvalue))