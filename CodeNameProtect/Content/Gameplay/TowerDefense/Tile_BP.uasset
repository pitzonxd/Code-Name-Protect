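; Tower defense grid tile actor that highlights by swapping its material and animating its mesh vertically.
; LightUp applies GridMat_NInv, then plays a timeline that offsets the Tile component upward from the actor's location.
; LightDown runs a second timeline in reverse with a downward offset, restoring GridMat_Inv when finished.
; BeginPlay stores the actor location in TmpLoc, but both animations read the live actor location instead.
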(event Custom|LightUp
  (bind _returnvalue (Transformation|GetActorLocation))
  (Rendering|Material|SetMaterial (Variables|Default|GetTile) 0 "/Game/testing/GridMat_NInv.GridMat_NInv")
  (bind _newtrack_0 (Timeline|LightUpDownAnimation PlayFromStart)
    (:Update
      (Transformation|SetWorldLocation (Variables|Default|GetTile) (Math|Vector|MakeVector (.x _returnvalue) (.y _returnvalue) (+ (.z _returnvalue) (* _newtrack_0 3e+01))) false false))))

(event Custom|LightDown
  (bind _returnvalue (Transformation|GetActorLocation))
  (bind _newtrack_0 (Timeline|Timeline_0 ReverseFromEnd)
    (:Update
      (Transformation|SetWorldLocation (Variables|Default|GetTile) (Math|Vector|MakeVector (.x _returnvalue) (.y _returnvalue) (- (.z _returnvalue) (* _newtrack_0 3e+01))) false false))
    (:Finished
      (Rendering|Material|SetMaterial (Variables|Default|GetTile) 0 "/Game/testing/GridMat_Inv.GridMat_Inv"))))

(event EventBeginPlay
  (Variables|Default|SettmpLoc (Transformation|GetActorLocation)))

(fn ConstructionScript)