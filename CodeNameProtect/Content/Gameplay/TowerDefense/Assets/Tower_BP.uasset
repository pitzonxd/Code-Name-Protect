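; Tower defense turret that damages the closest enemy within its damage radius, built on a parent placeable class.
; On placement it runs the parent logic, applies its material and sets its wall collision checker to overlap a custom trace channel.
; Each tick it gets the target from the player character's grid, line-traces toward it with a debug line, and applies frame-time-scaled damage if a standard enemy is hit.
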(event EventPlaceTarget
  ;[1 1 1] Place target
  (|CallParentFunction)
  (Rendering|Material|SetMaterial (Variables|Default|GetStaticMesh) 0 (Variables|Default|GetMaterial))
  (Collision|SetCollisionResponsetoChannel (Variables|Default|GetWallCollisionChecker) "ECC_GameTraceChannel1" "ECR_Overlap"))

(event EventTick
  (params (DeltaSeconds :type Float%20%28single-precision%29))
  (bind _returnvalue (Transformation|GetActorLocation))
  ;[1 1 1] Find closest enemy and start shooting
  (|CallParentFunction DeltaSeconds)
  (bind _aschar_emma (Utilities|Casting|CastToChar_Emma (Game|GetPlayerCharacter 0)))
  (bind _enemy (Default|GetClosestEnemytoTower (Variables|/Game/Gameplay/GeneralBPs/Char_Emma.Char_Emma_C|GetGridReference _aschar_emma) self (Variables|Default|GetdamageRadius)))
  (if (!= _enemy 0)
    (bind _outhit (Collision|LineTraceByChannel (Math|Vector|MakeVector (.x _returnvalue) (.y _returnvalue) 3e+02) (Math|Vector|MakeVector (.x (Transformation|GetActorLocation _enemy)) (.y (Transformation|GetActorLocation _enemy)) 1e+02) "TraceTypeQuery2" false 0 "ForOneFrame"))
    (bind _asstandard_enemy_bp (Utilities|Casting|CastToStandardEnemy_BP (.HitActor (Collision|BreakHitResult _outhit))))
    (Game|Damage|ApplyDamage _asstandard_enemy_bp (* DeltaSeconds (Variables|Default|GetdamageMultiplier)) 0 0)))

(fn ConstructionScript)