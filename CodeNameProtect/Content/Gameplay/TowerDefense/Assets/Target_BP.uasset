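; Tower-defense placeable target that previews placement validity, locks in as a pawn-blocking object and can be marked for destruction.
; Tick swaps materials by state and rejects placement when overlapping Char_Emma or another target, or blocking the path.
; Path blocking comes from the PathCheckingAI_BP CanReachTarget blackboard key.
; Destruction targeting spreads to directly overlapping targets only for Wall_BP, while untargeting always clears them.
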(event Custom|CheckPathBlocking
  (bind _returnvalue (Actor|GetActorOfClass "/Game/Gameplay/TowerDefense/PathCheckingAI/PathCheckingAI_BP.PathCheckingAI_BP_C"))
  (if (not (Variables|Default|Getplaced))
    (Variables|Default|SetblockingAI (not (ScalableFloat|GetValueasBool (AI|GetBlackboard _returnvalue) (Variables|Default|GetcanReachTarget))))))

(event Custom|PlaceTarget
  ;[1 1 1] Place Target down
  (if (Variables|Default|GetcanBePlaced)
    (Collision|SetCollisionResponsetoChannel (Variables|Target_BP_C|GetStaticMesh self) "ECC_Pawn" "ECR_Block")
    (Variables|Default|Setplaced true)))

(event EventTick
  (params (DeltaSeconds :type Float%20%28single-precision%29))
  (bind _staticmesh (Variables|Default|GetStaticMesh))
  (bind _staticmesh_2 (Variables|Default|GetStaticMesh))
  (CallFunction|CheckPathBlocking)
  (if (Variables|Default|GettargetedForDestruction)
    (Rendering|Material|SetMaterial _staticmesh_2 0 "/Game/Art/Material/BuildingSystem/Template/RedMaterial.RedMaterial")
    (elif (Variables|Default|Getplaced)
      (Rendering|Material|SetMaterial _staticmesh_2 0 "/Game/Geometry/Meshes/CubeMaterial.CubeMaterial")
      (elif (Variables|Default|GetblockingAI)
        (Rendering|Material|SetMaterial _staticmesh 0 "/Game/Art/Material/BuildingSystem/Template/RedMaterial.RedMaterial" :!label _label)
        (Variables|Default|SetcanBePlaced false)
        (elif (> (+ (Utilities|Array|Length (Collision|GetOverlappingActors "/Game/Gameplay/GeneralBPs/Char_Emma.Char_Emma_C" :!class /Script/Engine.Actor)) (Utilities|Array|Length (Collision|GetOverlappingActors "Target_BP_C" :!class /Script/Engine.Actor))) 0)
          (goto _label)
          (else
            (Rendering|Material|SetMaterial _staticmesh 0 "/Game/Art/Material/BuildingSystem/Template/BlueprintMaterial.BlueprintMaterial")
            (Variables|Default|SetcanBePlaced true)))))))

(fn ConstructionScript)

(fn TargetforDestruction
  (if (== (Utilities|GetClass self) "/Game/Gameplay/TowerDefense/Assets/Wall_BP.Wall_BP_C")
    (bind _allconnectedtargets (CallFunction|GetConnectedTargets))
    (for _array_element _allconnectedtargets
      (Variables|Target_BP_C|SettargetedForDestruction _array_element true)))
  (Variables|Default|SettargetedForDestruction true))

(fn UntargetforDestruction
  (bind _allconnectedtargets (CallFunction|GetConnectedTargets))
  (for _array_element _allconnectedtargets
    (Variables|Target_BP_C|SettargetedForDestruction _array_element false))
  (Variables|Default|SettargetedForDestruction false))

(fn GetConnectedTargets
  (for _array_element (Collision|GetOverlappingActors 0 :!class /Script/Engine.Actor)
    (bind _astarget_bp (Utilities|Casting|CastToTarget_BP _array_element))
    (Utilities|Array|Add (LocalVariables|GetConnectedTargetsTmp) _astarget_bp))
  (return (LocalVariables|GetConnectedTargetsTmp)))