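; A tower-defense trap placeable only on walls, which damages enemies entering its hitbox with spikes.
; While unplaced, it checks for overlapping Wall_BP actors, deferring to parent placement logic on a wall or turning red and blocking placement otherwise.
; A hitbox overlap damages the StandardEnemy_BP and starts a spike timeline.
; The same timeline reverses after the activation time, then re-arms the trap after a cooldown.
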(event OnComponentBeginOverlap(Hitbox)
  (params (OverlappedComponent :type Primitive%20Component%20Object%20Reference) (OtherActor :type Actor%20Object%20Reference) (OtherComp :type Primitive%20Component%20Object%20Reference) (OtherBodyIndex :type Integer) (bFromSweep :type Boolean) (SweepResult :type Hit%20Result%20Structure%20%28by%20ref%29))
  ;[1 1 1] Apply damage to overlaping enemy
  (if (Variables|Default|GetcanBeTriggered)
    (bind _asstandard_enemy_bp (Utilities|Casting|CastToStandardEnemy_BP OtherActor))
    (Game|Damage|ApplyDamage _asstandard_enemy_bp (Variables|Default|Getdamage) 0 0)
    (CallFunction|EnableTrap)))

(event Custom|EnableTrap
  ;[1 1 1] Enable Disable trap
  (Variables|Default|SetcanBeTriggered false)
  (Variables|Default|Setenabled true)
  (bind _newtrack_0 (Timeline|EnableDisableSpikes PlayFromStart)
    (:Update
      (Transformation|SetRelativeLocation (Variables|Default|GetSpikes) (Math|Vector|MakeVector 0.0 0.0 (+ (* _newtrack_0 5e+01) 3e+01)) false false))
    (:Finished
      (if (Variables|Default|Getenabled)
        (Utilities|FlowControl|Delay (Variables|Default|GetactivationTime))
        (CallFunction|DisableTrap)
        (else
          (Utilities|FlowControl|Delay (Variables|Default|Getcooldown))
          (Variables|Default|SetcanBeTriggered true))))))

(event Custom|DisableTrap
  ;[1 1 1] Enable Disable trap
  (Variables|Default|Setenabled false)
  (bind _newtrack_0 (Timeline|EnableDisableSpikes ReverseFromEnd)
    (:Update
      (Transformation|SetRelativeLocation (Variables|Default|GetSpikes) (Math|Vector|MakeVector 0.0 0.0 (+ (* _newtrack_0 5e+01) 3e+01)) false false))
    (:Finished
      (if (Variables|Default|Getenabled)
        (Utilities|FlowControl|Delay (Variables|Default|GetactivationTime))
        (CallFunction|DisableTrap)
        (else
          (Utilities|FlowControl|Delay (Variables|Default|Getcooldown))
          (Variables|Default|SetcanBeTriggered true))))))

(event EventTick
  (params (DeltaSeconds :type Float%20%28single-precision%29))
  ;[1 1 1] Can only be placed onto a wall
  ;;[1 1 1] CHANGED
  (if (Variables|Default|Getplaced)
    (|CallParentFunction DeltaSeconds)
    (else
      (Collision|SetCollisionResponsetoChannel (Variables|Default|GetWallCollisionChecker) "ECC_GameTraceChannel1" "ECR_Overlap")
      (if (> (Utilities|Array|Length (Collision|GetOverlappingActors (Variables|Default|GetWallCollisionChecker) "/Game/Gameplay/TowerDefense/Assets/Wall_BP.Wall_BP_C" :!class /Script/Engine.PrimitiveComponent)) 0)
        (Collision|SetCollisionResponsetoChannel (Variables|Default|GetWallCollisionChecker) "ECC_GameTraceChannel1" "ECR_Ignore")
        (|CallParentFunction DeltaSeconds)
        (else
          (Rendering|Material|SetMaterial (Variables|Default|GetStaticMesh) 0 "/Game/Art/Material/BuildingSystem/Template/RedMaterial.RedMaterial")
          (Variables|Default|SetcanBePlaced false))))))

(event EventPlaceTarget
  (bind _material (Variables|Default|GetMaterial))
  ;[1 1 1] Set material when placed
  (|CallParentFunction)
  (Rendering|Material|SetMaterial (Variables|Default|GetStaticMesh) 0 _material)
  (Rendering|Material|SetMaterial (Variables|Default|GetSpikes) 0 _material)
  (Collision|SetCollisionResponsetoChannel (Variables|Default|GetWallCollisionChecker) "ECC_GameTraceChannel1" "ECR_Overlap"))

(event EventBeginPlay
  ;[1 1 1] Set rotation, so that the player sees the front of the trap when spawned
  (|CallParentFunction))

(fn ConstructionScript
  (Variables|Default|SetTrapLocation (Transformation|GetWorldLocation (Variables|Default|GetSpikes))))