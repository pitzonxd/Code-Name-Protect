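; Tower defense spawner actor that releases waves of standard enemies at its own location.
; SpawnEnemies sets the wave size and starts a looping timer at the given delay.
; Each tick spawns a StandardEnemy_BP pawn running Enemy_BT until the count is reached, then pauses the timer and resets the spawned counter.
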(event Custom|SpawnEnemies
  (params (Number :type Integer) (DelayBetweenSpawning :type Float%20%28single-precision%29))
  (Variables|Default|SetEnemiesToSpawn Number)
  (bind _returnvalue (Utilities|Time|SetTimerbyEvent (delegate Custom|Spawn) DelayBetweenSpawning true))
  (Variables|Default|SetTimerHandle _returnvalue))

(event Custom|Spawn
  (if (>= (Variables|Default|GetSpawnedEnemies) (Variables|Default|GetEnemiesToSpawn))
    (Utilities|Time|PauseTimerbyHandle (Variables|Default|GetTimerHandle))
    (Variables|Default|SetSpawnedEnemies 0)
    (else
      (Math|Integer|IncrementInt (Variables|Default|GetSpawnedEnemies)
        (:%20%20
          (AI|SpawnAIFromClass "/Game/Gameplay/TowerDefense/Enemies/StandardEnemy_BP.StandardEnemy_BP_C" "/Game/Gameplay/TowerDefense/Enemies/Enemy_BT.Enemy_BT" (Transformation|GetActorLocation) "0, 0, 0" false 0))))))

(fn ConstructionScript)